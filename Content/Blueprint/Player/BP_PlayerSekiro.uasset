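; Sekiro-style player Blueprint that binds Enhanced Input to movement, jump, dash, attack, guard, gourd healing and lock-on.
; BeginPlay adds the mapping context, and input events forward to handlers defined outside this file.
; Dash, attack and guard pass hold time on Triggered and Completed.
; Mouse turns the camera, or searches for another target while locked on; nonzero forward/back input also feeds MoveRight.
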(event EventBeginPlay
  (Pawn|Input|AddControllerPitchInput 3.0)
  (Input|AddMappingContext (PlayerController|LocalPlayerSubsystems|GetEnhancedInputLocalPlayerSubsystem (Game|GetPlayerController 0)) "/Game/Blueprint/Input/EI_PlayerInput.EI_PlayerInput" 0 "(bIgnoreAllPressedKeysUntilRelease=True,bForceImmediately=False)"))

(event Collision|EventActorBeginOverlap
  (params (OtherActor :type Actor%20Object%20Reference)))

(event EventTick
  (params (DeltaSeconds :type Float%20%28single-precision%29)))

(event Input|EnhancedActionEvents|EnhancedInputActionEI_PlayerMoveFB
  (params (ActionValue :type Float%20%28double-precision%29) (ElapsedSeconds :type Float%20%28double-precision%29) (TriggeredSeconds :type Float%20%28double-precision%29) (InputAction :type Input%20Action%20Object%20Reference :default "/Game/Blueprint/Input/EI_PlayerMoveFB.EI_PlayerMoveFB"))
  (:Triggered
    (Variables|Default|SetbInputWASD true)
    (Class|PlayerSekiro|MoveForward ActionValue)
    (if (!= (stale Input|EnhancedActionEvents|EnhancedInputActionEI_PlayerMoveLR ActionValue) 0.0)
      (Class|PlayerSekiro|MoveRight (stale Input|EnhancedActionEvents|EnhancedInputActionEI_PlayerMoveLR ActionValue))))
  (:Completed
    (Variables|Default|SetbInputWASD false)
    (Class|PlayerSekiro|MoveForward 0.0)))

(event Input|EnhancedActionEvents|EnhancedInputActionEI_PlayerMoveLR
  (params (ActionValue :type Float%20%28double-precision%29) (ElapsedSeconds :type Float%20%28double-precision%29) (TriggeredSeconds :type Float%20%28double-precision%29) (InputAction :type Input%20Action%20Object%20Reference :default "/Game/Blueprint/Input/EI_PlayerMoveLR.EI_PlayerMoveLR"))
  (:Triggered
    (Variables|Default|SetbInputWASD true)
    (Class|PlayerSekiro|MoveRight ActionValue))
  (:Completed
    (Variables|Default|SetbInputWASD false)
    (Class|PlayerSekiro|MoveRight 0.0)))

(event Input|EnhancedActionEvents|EnhancedInputActionEI_PlayerJump
  (params (ActionValue :type Boolean) (ElapsedSeconds :type Float%20%28double-precision%29) (TriggeredSeconds :type Float%20%28double-precision%29) (InputAction :type Input%20Action%20Object%20Reference :default "/Game/Blueprint/Input/EI_PlayerJump.EI_PlayerJump"))
  (:Started
    (Class|PlayerSekiro|PlayerJump)))

(event Input|EnhancedActionEvents|EnhancedInputActionEI_PlayerDash
  (params (ActionValue :type Boolean) (ElapsedSeconds :type Float%20%28double-precision%29) (TriggeredSeconds :type Float%20%28double-precision%29) (InputAction :type Input%20Action%20Object%20Reference :default "/Game/Blueprint/Input/EI_PlayerDash.EI_PlayerDash"))
  (:Triggered
    (Class|PlayerSekiro|TriggeredPlayerDash ActionValue TriggeredSeconds))
  (:Started
    (Class|PlayerSekiro|StartedPlayerDash))
  (:Completed
    (Class|PlayerSekiro|TriggeredPlayerDash ActionValue TriggeredSeconds)))

(event Input|EnhancedActionEvents|EnhancedInputActionEI_PlayerMouseTurn
  (params (ActionValue :type Vector%202D%20Structure) (ElapsedSeconds :type Float%20%28double-precision%29) (TriggeredSeconds :type Float%20%28double-precision%29) (InputAction :type Input%20Action%20Object%20Reference :default "/Game/Blueprint/Input/EI_PlayerMouseTurn.EI_PlayerMouseTurn"))
  (:Triggered
    (if (Variables|Default|GetbLockOn)
      (Class|PlayerSekiro|ResearchLockonTarget (.x ActionValue))
      (else
        (Pawn|Input|AddControllerYawInput (.x ActionValue))
        (Pawn|Input|AddControllerPitchInput (* (.y ActionValue) -1.0))))))

(event Input|EnhancedActionEvents|EnhancedInputActionEI_PlayerLockOn
  (params (ActionValue :type Boolean) (ElapsedSeconds :type Float%20%28double-precision%29) (TriggeredSeconds :type Float%20%28double-precision%29) (InputAction :type Input%20Action%20Object%20Reference :default "/Game/Blueprint/Input/EI_PlayerLockOn.EI_PlayerLockOn"))
  (:Started
    (Class|PlayerSekiro|LockonTarget)))

(event Input|EnhancedActionEvents|EnhancedInputActionEI_PlayerAttack
  (params (ActionValue :type Boolean) (ElapsedSeconds :type Float%20%28double-precision%29) (TriggeredSeconds :type Float%20%28double-precision%29) (InputAction :type Input%20Action%20Object%20Reference :default "/Game/Blueprint/Input/EI_PlayerAttack.EI_PlayerAttack"))
  (:Triggered
    (Class|PlayerSekiro|TriggeredPlayerAttack ActionValue TriggeredSeconds))
  (:Started
    (Class|PlayerSekiro|StartedPlayerAttack))
  (:Completed
    (Class|PlayerSekiro|TriggeredPlayerAttack ActionValue TriggeredSeconds)))

(event Input|EnhancedActionEvents|EnhancedInputActionEI_PlayerGuard
  (params (ActionValue :type Boolean) (ElapsedSeconds :type Float%20%28double-precision%29) (TriggeredSeconds :type Float%20%28double-precision%29) (InputAction :type Input%20Action%20Object%20Reference :default "/Game/Blueprint/Input/EI_PlayerGuard.EI_PlayerGuard"))
  (:Triggered
    (Class|PlayerSekiro|TriggeredPlayerGuard ActionValue TriggeredSeconds))
  (:Started
    (Class|PlayerSekiro|StartedPlayerGuard))
  (:Completed
    (Class|PlayerSekiro|TriggeredPlayerGuard ActionValue TriggeredSeconds)))

(event Input|EnhancedActionEvents|EnhancedInputActionEI_PlayerHeal
  (params (ActionValue :type Boolean) (ElapsedSeconds :type Float%20%28double-precision%29) (TriggeredSeconds :type Float%20%28double-precision%29) (InputAction :type Input%20Action%20Object%20Reference :default "/Game/Blueprint/Input/EI_PlayerHeal.EI_PlayerHeal"))
  (:Started
    (Class|PlayerSekiro|DrinkGourd)))

(fn ConstructionScript)