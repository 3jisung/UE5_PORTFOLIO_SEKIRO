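; Sequencer event Blueprint for the Genichiro phase 2 cutscene, finding the boss by actor tag.
; On play, it places boss and player at fixed transforms, removes player input, hides the HUD and lock-on icon.
; Phase events set the boss's intro animation states, and a sound event calls the game mode.
; On end, it restores input and HUD, restores lock-on or faces the boss, then fades a transition widget.
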(event Custom|PlaySequence
  (bind _returnvalue (Game|GetPlayerCharacter 0))
  (bind _returnvalue_2 (Game|GetPlayerController 0))
  (Utilities|FlowControl|Sequence
    (:then_0
      (bind _outactors (Actor|GetAllActorswithTag "아시나 겐이치로"))
      (if (!= (Utilities|Array|Get(acopy) _outactors) 0)
        (Transformation|SetActorLocation (Utilities|Array|Get(acopy) _outactors) "-4766.614491,15950.466404,-6286.991371" false false)
        (Transformation|SetActorRotation (Utilities|Array|Get(acopy) _outactors) "0.000000,-75.000000,0.000000")
        (bind _asmonster (Utilities|Casting|CastToMonster (Utilities|Array|Get(acopy) _outactors)))
        (if (!= (UserInterface|GetWidget (Variables|/Script/UE5_PORTFOLIO_SEKIRO.Monster|GetLockOnWidgetComponent _asmonster)) 0)
          (Variables|Default|SetbLockOnIcon true)
          (Class|Monster|LockonIcononOff _asmonster false)
          (else
            (Variables|Default|SetbLockOnIcon false)))))
    (:then_1
      (Transformation|SetActorLocation _returnvalue "-4400.000000,15110.000000,-6290.000000" false false)
      (Transformation|SetActorRotation _returnvalue "0.000000,110.000000,0.000000"))
    (:then_2
      (Input|RemoveMappingContext (PlayerController|LocalPlayerSubsystems|GetEnhancedInputLocalPlayerSubsystem _returnvalue_2) "/Game/Blueprint/Input/EI_PlayerInput.EI_PlayerInput" "(bIgnoreAllPressedKeysUntilRelease=True,bForceImmediately=False)")
      (bind _asglobal_hud (Utilities|Casting|CastToGlobalHUD (HUD|GetHUD _returnvalue_2)))
      (bind _returnvalue_3 (Class|GlobalHUD|GetMainWidget _asglobal_hud))
      (Variables|/Script/UMG.Widget|SetVisibility _returnvalue_3 "Hidden"))))

(event Custom|Phase2_1
  (bind _outactors (Actor|GetAllActorswithTag "아시나 겐이치로"))
  (if (!= (Utilities|Array|Get(acopy) _outactors) 0)
    (bind _asglobal_character (Utilities|Casting|CastToGlobalCharacter (Utilities|Array|Get(acopy) _outactors)))
    (Variables|/Script/UE5_PORTFOLIO_SEKIRO.GlobalCharacter|SetAniState _asglobal_character (Math|Conversions|ToInteger(Byte) (Utilities|Enum|LiteralenumGenichiroState "Phase2Intro1")))))

(event Custom|Phase2_2
  (bind _outactors (Actor|GetAllActorswithTag "아시나 겐이치로"))
  (if (!= (Utilities|Array|Get(acopy) _outactors) 0)
    (bind _asglobal_character (Utilities|Casting|CastToGlobalCharacter (Utilities|Array|Get(acopy) _outactors)))
    (Variables|/Script/UE5_PORTFOLIO_SEKIRO.GlobalCharacter|SetAniState _asglobal_character (Math|Conversions|ToInteger(Byte) (Utilities|Enum|LiteralenumGenichiroState "Phase2Intro2")))))

(event Custom|EndSquence
  (bind _returnvalue (Game|GetPlayerController 0))
  (Utilities|FlowControl|Sequence
    (:then_0
      (Input|AddMappingContext (PlayerController|LocalPlayerSubsystems|GetEnhancedInputLocalPlayerSubsystem _returnvalue) "/Game/Blueprint/Input/EI_PlayerInput.EI_PlayerInput" 0 "(bIgnoreAllPressedKeysUntilRelease=True,bForceImmediately=False)")
      (bind _asglobal_hud (Utilities|Casting|CastToGlobalHUD (HUD|GetHUD _returnvalue)))
      (bind _returnvalue_2 (Class|GlobalHUD|GetMainWidget _asglobal_hud))
      (Variables|/Script/UMG.Widget|SetVisibility _returnvalue_2 "Visible"))
    (:then_1
      (bind _outactors (Actor|GetAllActorswithTag "아시나 겐이치로"))
      (if (!= (Utilities|Array|Get(acopy) _outactors) 0)
        (bind _asmonster (Utilities|Casting|CastToMonster (Utilities|Array|Get(acopy) _outactors)))
        (if (Variables|Default|GetbLockOnIcon)
          (Class|Monster|LockonIcononOff _asmonster true)
          (else
            (Pawn|SetControlRotation _returnvalue (Math|Rotator|FindLookatRotation (Transformation|GetActorLocation _returnvalue) (Transformation|GetActorLocation (Utilities|Array|Get(acopy) _outactors))))))))
    (:then_2
      (bind _returnvalue_3 (UserInterface|CreateWidget "/Game/Blueprint/Global/WBP_SceneTransition.WBP_SceneTransition_C"))
      (UserInterface|Viewport|AddtoViewport _returnvalue_3 0)
      (Class|FadeinOutWidget|SetCanvasRenderOpacity _returnvalue_3 1.0)
      (Class|FadeinOutWidget|FadeOut _returnvalue_3 true))))

(event Custom|PlaySound
  (bind _asglobal_game_mode (Utilities|Casting|CastToGlobalGameMode (Game|GetGameMode)))
  (Class|GlobalGameMode|ModifySound _asglobal_game_mode 1 0.0))