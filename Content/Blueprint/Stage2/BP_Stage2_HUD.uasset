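; Stage 2 HUD Blueprint that sets up the stage's UI and opening transition when play begins.
; BeginPlay creates and registers the main widget, then lays a fully opaque scene transition widget above it.
; After a short delay it has GlobalGameMode play a sound and fades the transition out, both only if the game mode cast succeeds.
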(event EventBeginPlay
  (bind _returnvalue (UserInterface|CreateWidget "/Game/Blueprint/Player/UI/WBP_MainWidget.WBP_MainWidget_C"))
  (UserInterface|Viewport|AddtoViewport _returnvalue 0)
  (Class|GlobalHUD|SetMainWidget _returnvalue)
  (bind _returnvalue_2 (UserInterface|CreateWidget "/Game/Blueprint/Global/WBP_SceneTransition.WBP_SceneTransition_C"))
  (UserInterface|Viewport|AddtoViewport _returnvalue_2 1)
  (Class|FadeinOutWidget|SetCanvasRenderOpacity _returnvalue_2 1.0)
  (Utilities|FlowControl|Delay 0.5)
  (bind _asglobal_game_mode (Utilities|Casting|CastToGlobalGameMode (Game|GetGameMode)))
  (Class|GlobalGameMode|PlaySound _asglobal_game_mode)
  (Class|FadeinOutWidget|FadeOut _returnvalue_2 true))

(event Collision|EventActorBeginOverlap
  (params (OtherActor :type Actor%20Object%20Reference)))

(event EventTick
  (params (DeltaSeconds :type Float%20%28single-precision%29)))

(fn ConstructionScript)