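; BP_TitleHUD sets up the title screen UI when play begins.
; BeginPlay adds WBP_TitleScreen to the viewport, then layers WBP_SceneTransition above it to play a fade-in, removing it after a one-second delay.
; It also switches the player controller to UI-only input focused on the title screen and shows the mouse cursor.
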(event EventBeginPlay
  (bind _returnvalue (Game|GetPlayerController 0))
  (Utilities|FlowControl|Sequence
    (:then_0
      (bind _returnvalue_2 (UserInterface|CreateWidget "/Game/Blueprint/Title/WBP_TitleScreen.WBP_TitleScreen_C"))
      (UserInterface|Viewport|AddtoViewport _returnvalue_2 0))
    (:then_1
      (bind _returnvalue_3 (UserInterface|CreateWidget "/Game/Blueprint/Global/WBP_SceneTransition.WBP_SceneTransition_C"))
      (UserInterface|Viewport|AddtoViewport _returnvalue_3 1)
      (Class|FadeinOutWidget|Fadein _returnvalue_3)
      (Utilities|FlowControl|Delay 1.0)
      (Widget|RemovefromParent _returnvalue_3))
    (:then_2
      (Input|SetInputModeUIOnly _returnvalue _returnvalue_2 "DoNotLock" false)
      (Variables|/Script/Engine.PlayerController|SetbShowMouseCursor _returnvalue true))))

(event Collision|EventActorBeginOverlap
  (params (OtherActor :type Actor%20Object%20Reference)))

(event EventTick
  (params (DeltaSeconds :type Float%20%28single-precision%29)))

(fn ConstructionScript)