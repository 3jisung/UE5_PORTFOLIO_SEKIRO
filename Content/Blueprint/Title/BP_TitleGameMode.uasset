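; Game mode for the title screen that prepares the player for menu interaction.
; BeginPlay switches the first player controller to UI-only input and shows the mouse cursor.
; A disconnected, never-executed chain would create the title screen widget, overlay a scene transition widget, play a sound with a delayed fade-in, then remove the overlay.
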(event EventBeginPlay
  (bind _returnvalue (Game|GetPlayerController 0))
  (Input|SetInputModeUIOnly _returnvalue 0 "DoNotLock" false)
  (Variables|/Script/Engine.PlayerController|SetbShowMouseCursor _returnvalue true))

(event EventTick
  (params (DeltaSeconds :type Float%20%28single-precision%29)))

(fn ConstructionScript)